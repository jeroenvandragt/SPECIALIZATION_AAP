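; Road tile for a Holland-themed level that dresses itself with random props and extends the track as the player advances.
; On BeginPlay, SpawnObstacles places a random house on each sidewalk, mirroring the left one with negative X scale, and a random obstacle at each of two road points.
; When the Player overlaps Collision, it asks FreeMonkeyGameMode to spawn another tile unless the goal is reached.
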(event `self.Collision.OnComponentBeginOverlap`
  (params (OtherActor :type "Actor Object Reference") (OtherComp :type "PrimitiveComponent Object Reference") (OtherBodyIndex :type Integer) (bFromSweep :type Boolean) (SweepResult :type "HitResult Structure (by ref)"))
  (cast `/Game/Player` OtherActor)
  (bind _asfree_monkey_game_mode (cast `/Game/FreeMonkeyGameMode` (`GameplayStatics.GetGameMode`)))
  (if (not (`/Game/FreeMonkeyGameMode.IsGoalReached` _asfree_monkey_game_mode))
    (`/Game/FreeMonkeyGameMode.Spawn_Tile` _asfree_monkey_game_mode)
    (`KismetSystemLibrary.PrintString` "New tile spawned.")))

(event `self.ReceiveBeginPlay`
  (`self.SpawnObstacles`))

(fn `SpawnObstacles`
  (bind _roadobstacles (`self.RoadObstacles`))
  (bind _houses (`self.Houses`))
  (bind _houses_2 (`self.Houses`))
  (bind _roadobstacles_2 (`self.RoadObstacles`))
  (bind (_returnvalue_location _returnvalue_rotation) (`KismetMathLibrary.BreakTransform` (`SceneComponent.K2_GetComponentToWorld` (`self.RightRoad`))))
  (bind (_returnvalue_location_2 _returnvalue_rotation_2) (`KismetMathLibrary.BreakTransform` (`SceneComponent.K2_GetComponentToWorld` (`self.LeftRoad`))))
  (`|ExecutionSequence`
    (:`then_0`
      (`|SpawnActorFromClass` (`KismetArrayLibrary.Array_Get` _houses_2 (`KismetMathLibrary.RandomInteger` (`KismetArrayLibrary.Array_Length` _houses_2))) (`KismetMathLibrary.MakeTransform` (`SceneComponent.K2_GetComponentLocation` (`self.RightSideWalkSpawnPoint`))) "Undefined" "OverrideRootScale")
      (`SceneComponent.K2_AttachTo` (`self.RightSideWalkSpawnPoint`) null "None" "KeepRelativeOffset" true))
    (:`then_1`
      (`|SpawnActorFromClass` (`KismetArrayLibrary.Array_Get` _houses (`KismetMathLibrary.RandomInteger` (`KismetArrayLibrary.Array_Length` _houses))) (`KismetMathLibrary.MakeTransform` (`SceneComponent.K2_GetComponentLocation` (`self.LeftSideWalkSpawnPoint`)) (struct) (-1.0 1.0 1.0)) "Undefined" "OverrideRootScale")
      (`SceneComponent.K2_AttachTo` (`self.LeftSideWalkSpawnPoint`) null "None" "KeepRelativeOffset" true))
    (:`then_2`
      (`|SpawnActorFromClass` (`KismetArrayLibrary.Array_Get` _roadobstacles (`KismetMathLibrary.RandomInteger` (`KismetArrayLibrary.Array_Length` _roadobstacles))) (`KismetMathLibrary.MakeTransform` _returnvalue_location_2 _returnvalue_rotation_2) "Undefined" "OverrideRootScale"))
    (:`then_3`
      (`|SpawnActorFromClass` (`KismetArrayLibrary.Array_Get` _roadobstacles_2 (`KismetMathLibrary.RandomInteger` (`KismetArrayLibrary.Array_Length` _roadobstacles_2))) (`KismetMathLibrary.MakeTransform` _returnvalue_location _returnvalue_rotation) "Undefined" "OverrideRootScale"))))

(fn `UserConstructionScript`)