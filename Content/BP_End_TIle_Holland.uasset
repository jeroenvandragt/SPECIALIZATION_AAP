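; End tile actor, apparently for a Holland level, that finishes the match when the player reaches it.
; On BeginPlay it spawns a BP_Reza actor at the location and rotation of its SpawnAnimalPosition component.
; Overlapping EndTrigger calls EndMatch on the game mode, with the player identified by an object name starting with "Player" instead of a cast.
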(event `self.EndTrigger.OnComponentBeginOverlap`
  (params (OtherActor :type "Actor Object Reference") (OtherComp :type "PrimitiveComponent Object Reference") (OtherBodyIndex :type Integer) (bFromSweep :type Boolean) (SweepResult :type "HitResult Structure (by ref)"))
  (if (== (`KismetStringLibrary.FindSubstring` (`KismetSystemLibrary.GetObjectName` OtherActor) "Player") 0)
    (`GameMode.EndMatch` (`GameplayStatics.GetGameMode`))))

(event `self.ReceiveBeginPlay`
  (bind _spawnanimalposition (`self.SpawnAnimalPosition`))
  (`|SpawnActorFromClass` "/Game/BP_Reza.BP_Reza_C" (`KismetMathLibrary.MakeTransform` (`SceneComponent.K2_GetComponentLocation` _spawnanimalposition) (`SceneComponent.K2_GetComponentRotation` _spawnanimalposition)) "Undefined" "OverrideRootScale"))

(fn `UserConstructionScript`)